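; Actor that logs right-leg thigh, calf and foot angles for a teacher and a subject to a CSV file.
; On BeginPlay it names the file after the animation assigned to a found actor's skeletal mesh.
; Each Tick it reads the angles from BP_DisplayAngle and appends them with elapsed time to that file in the project directory.
; DataNames prefixes the first write and is then cleared, serving as a one-time header.
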(event EventBeginPlay
  (bind _returnvalue (Actor|GetActorOfClass 0))
  (bind _output_get (Variables|Default|SetFileName (Utilities|GetDisplayName (.AnimToPlay (Utilities|Struct|BreakSingleAnimationPlayData (Variables|/Script/Engine.SkeletalMeshComponent|GetAnimationData (Variables|/Script/Engine.SkeletalMeshActor|GetSkeletalMeshComponent _returnvalue))))))))

(event EventTick
  (params (DeltaSeconds :type Float%20%28single-precision%29))
  (bind _returnvalue (Actor|GetActorOfClass "/Game/Blueprints/BP_DisplayAngle.BP_DisplayAngle_C"))
  (for _index (range 0 0)
    (Class|VictoryBPFunctionLibrary|FileIOSaveStringTexttoFile (Class|KismetSystemLibrary|GetProjectDirectory) (Utilities|String|Append (stale EventBeginPlay _output_get) ".csv") (Utilities|String|Append (Variables|Default|GetDataNames) "" (Utilities|String|ToString(Float) (Actor|GetGameTimeSinceCreation self)) "," (Utilities|String|ToString(Float) (Variables|/Game/Blueprints/BP_DisplayAngle.BP_DisplayAngle_C|GetAngleOfThigh_r_Teacher (Utilities|Array|Get(acopy) (Utilities|Array|MakeArray _returnvalue)))) "," (Utilities|String|ToString(Float) (Variables|/Game/Blueprints/BP_DisplayAngle.BP_DisplayAngle_C|GetAngleOfThigh_r_Subject (Utilities|Array|Get(acopy) (Utilities|Array|MakeArray _returnvalue)))) "," (Utilities|String|ToString(Float) (Variables|/Game/Blueprints/BP_DisplayAngle.BP_DisplayAngle_C|GetAngleOfCalf_r_Teacher (Utilities|Array|Get(acopy) (Utilities|Array|MakeArray _returnvalue)))) "," (Utilities|String|ToString(Float) (Variables|/Game/Blueprints/BP_DisplayAngle.BP_DisplayAngle_C|GetAngleOfCalf_r_Subject (Utilities|Array|Get(acopy) (Utilities|Array|MakeArray _returnvalue)))) "," (Utilities|String|ToString(Float) (Variables|/Game/Blueprints/BP_DisplayAngle.BP_DisplayAngle_C|GetAngleOfFoot_r_Teacher (Utilities|Array|Get(acopy) (Utilities|Array|MakeArray _returnvalue)))) "," (Utilities|String|ToString(Float) (Variables|/Game/Blueprints/BP_DisplayAngle.BP_DisplayAngle_C|GetAngleOfFoot_r_Subject (Utilities|Array|Get(acopy) (Utilities|Array|MakeArray _returnvalue)))) ",") true true))
  (Variables|Default|SetDataNames "")
  (Class|VictoryBPFunctionLibrary|FileIOSaveStringTexttoFile (Class|KismetSystemLibrary|GetProjectDirectory) (Utilities|String|Append (stale EventBeginPlay _output_get) ".csv") (Utilities|String|Append (Variables|Default|GetDataNames) "" (Utilities|String|ToString(Float) (Actor|GetGameTimeSinceCreation self)) "," (Utilities|String|ToString(Float) (Variables|/Game/Blueprints/BP_DisplayAngle.BP_DisplayAngle_C|GetAngleOfThigh_r_Teacher (Utilities|Array|Get(acopy) (Utilities|Array|MakeArray _returnvalue)))) "," (Utilities|String|ToString(Float) (Variables|/Game/Blueprints/BP_DisplayAngle.BP_DisplayAngle_C|GetAngleOfThigh_r_Subject (Utilities|Array|Get(acopy) (Utilities|Array|MakeArray _returnvalue)))) "," (Utilities|String|ToString(Float) (Variables|/Game/Blueprints/BP_DisplayAngle.BP_DisplayAngle_C|GetAngleOfCalf_r_Teacher (Utilities|Array|Get(acopy) (Utilities|Array|MakeArray _returnvalue)))) "," (Utilities|String|ToString(Float) (Variables|/Game/Blueprints/BP_DisplayAngle.BP_DisplayAngle_C|GetAngleOfCalf_r_Subject (Utilities|Array|Get(acopy) (Utilities|Array|MakeArray _returnvalue)))) "," (Utilities|String|ToString(Float) (Variables|/Game/Blueprints/BP_DisplayAngle.BP_DisplayAngle_C|GetAngleOfFoot_r_Teacher (Utilities|Array|Get(acopy) (Utilities|Array|MakeArray _returnvalue)))) "," (Utilities|String|ToString(Float) (Variables|/Game/Blueprints/BP_DisplayAngle.BP_DisplayAngle_C|GetAngleOfFoot_r_Subject (Utilities|Array|Get(acopy) (Utilities|Array|MakeArray _returnvalue)))) ",") true true))

(fn ConstructionScript)