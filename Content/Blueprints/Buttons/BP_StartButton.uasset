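; BP_StartButton is a focusable button that spawns a Ball actor at a fixed location when released.
; A ButtonComponent drives the MovingVisuals mesh and raises press, release, focus and enable events, with sounds played on press and release.
; On BeginPlay it creates a dynamic material and caches its Base Color.
; UpdateButtonColor then grays the button when disabled, brightens it when focused, or restores that color otherwise.
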(event OnButtonPressed(ButtonComponent)
  (params (Button :type Uxt%20Pressable%20Button%20Component%20Object%20Reference) (Pointer :type Uxt%20Pointer%20Component%20Object%20Reference))
  ;[1 1 1] Play sound on press
  (Audio|PlaySound2D (Variables|Button|GetPressedSound) 1.0 1.0 0.0 0 0))

(event OnButtonReleased(ButtonComponent)
  (params (Button :type Uxt%20Pressable%20Button%20Component%20Object%20Reference) (Pointer :type Uxt%20Pointer%20Component%20Object%20Reference))
  ;[1 1 1] Play sound on release
  (Audio|PlaySound2D (Variables|Button|GetReleasedSound) 1.0 1.0 0.0 0 0)
  (Game|SpawnActorfromClass "/Game/Blueprints/Ball.Ball_C" (Math|Conversions|ToTransform(Vector) "200.000000, 0,300.000000") "Undefined" 0 0))

(event OnBeginFocus(ButtonComponent)
  (params (Button :type Uxt%20Pressable%20Button%20Component%20Object%20Reference) (Pointer :type Uxt%20Pointer%20Component%20Object%20Reference) (bWasAlreadyFocused :type Boolean))
  (if (not bWasAlreadyFocused)
    (CallFunction|UpdateButtonColor)))

(event OnEndFocus(ButtonComponent)
  (params (Button :type Uxt%20Pressable%20Button%20Component%20Object%20Reference) (Pointer :type Uxt%20Pointer%20Component%20Object%20Reference) (bIsStillFocused :type Boolean))
  (if (not bIsStillFocused)
    (CallFunction|UpdateButtonColor)))

(event OnButtonEnabled(ButtonComponent)
  (params (Button :type Uxt%20Pressable%20Button%20Component%20Object%20Reference))
  (CallFunction|UpdateButtonColor))

(event OnButtonDisabled(ButtonComponent)
  (params (Button :type Uxt%20Pressable%20Button%20Component%20Object%20Reference))
  (CallFunction|UpdateButtonColor))

(event EventBeginPlay
  (bind _movingvisuals (Variables|Default|GetMovingVisuals))
  (Class|UxtPressableButtonComponent|SetVisuals (Variables|Default|GetButtonComponent) (Variables|Default|GetMovingVisuals))
  ;[1 1 1] Create a dynamic material instance so we can update it to reflect button state
  (bind _returnvalue (Rendering|Material|CreateDynamicMaterialInstance _movingvisuals 0 (Rendering|Material|GetMaterial _movingvisuals 0) "None" :!class /Script/Engine.PrimitiveComponent))
  ;[1 1 1] Store initial base color
  (bind _returnvalue_2 (Rendering|Material|GetVectorParameterValue _returnvalue "Base Color" :!class /Script/Engine.MaterialInstanceDynamic))
  (Variables|Default|SetBaseColor _returnvalue_2))

(fn ConstructionScript)

(fn UpdateButtonColor
  (switch Utilities|FlowControl|Switch|SwitchonEUxtButtonState (Class|UxtPressableButtonComponent|GetState (Variables|Default|GetButtonComponent))
    (:Default
      ;[1 1 1] Set original base color
      (Rendering|Material|SetVectorParameterValueonMaterials (Variables|Default|GetMovingVisuals) "Base Color" (Math|Conversions|ToVector(LinearColor) (Variables|Default|GetBaseColor))))
    (:Disabled
      ;[1 1 1] Gray out button when disabled
      (Rendering|Material|SetVectorParameterValueonMaterials (Variables|Default|GetMovingVisuals) "Base Color" (Math|Conversions|ToVector(LinearColor) "(R=0.250000,G=0.250000,B=0.250000,A=1.000000)")))
    (:Focused
      ;[1 1 1] Lighten base color when focused
      (Rendering|Material|SetVectorParameterValueonMaterials (Variables|Default|GetMovingVisuals) "Base Color" (Math|Conversions|ToVector(LinearColor) (* (Variables|Default|GetBaseColor) 2.0))))))