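; Actor that exports right thigh, calf and foot angles to a CSV during a frame window around an animation's impact frame.
; BeginPlay names the file after the Sub actor's animation and writes the DataNames text to it.
; Start and End convert frames to game-time bounds.
; Within that window, each Tick appends a timing label, relative time and the subject angles read from BP_DisplayAngle.
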(event EventBeginPlay
  ;[1 1 1] ファイル名をつける
  (bind _returnvalue (Actor|GetActorOfClass "/Game/Blueprints/Sub.Sub_C"))
  (bind _output_get (Variables|Default|SetFile%20Name (Utilities|GetDisplayName (.AnimToPlay (Utilities|Struct|BreakSingleAnimationPlayData (Variables|/Script/Engine.SkeletalMeshComponent|GetAnimationData (Variables|/Script/Engine.SkeletalMeshActor|GetSkeletalMeshComponent _returnvalue)))))))
  (Class|VictoryBPFunctionLibrary|FileIOSaveStringTexttoFile (Class|KismetSystemLibrary|GetProjectDirectory) (Utilities|String|Append _output_get ".csv") (Variables|Default|GetDataNames) true true))

(event EventTick
  (params (DeltaSeconds :type Float%20%28single-precision%29))
  (bind _impactframe (Variables|Default|GetImpactFrame))
  (bind _animationfps (Variables|Default|GetAnimationFPS))
  (bind _impactframe_2 (Variables|Default|GetImpactFrame))
  (bind _animationfps_2 (Variables|Default|GetAnimationFPS))
  (bind _framesbeforeimpact (Variables|Default|GetFramesBeforeImpact))
  (bind _returnvalue (Math|Conversions|ToFloat(Integer) _animationfps_2))
  (bind _returnvalue_2 (Actor|GetActorOfClass "/Game/Blueprints/BP_DisplayAngle.BP_DisplayAngle_C"))
  ;[1 1 1] Tickごとの繰り返し処理
  (if (stale _isstarted)
    (bind _is_ended (CallFunction|End _impactframe _animationfps))
    (if _is_ended
      (Class|VictoryBPFunctionLibrary|FileIOSaveStringTexttoFile (Class|KismetSystemLibrary|GetProjectDirectory) (Utilities|String|Append (stale EventBeginPlay _output_get) ".csv") (Utilities|String|Append (Utilities|String|Append (Utilities|String|ToString(Integer) _impactframe_2) "-" (Utilities|String|ToString(Float) _framesbeforeimpact) "/" (Utilities|String|ToString(Integer) _animationfps_2)) "," (Utilities|String|ToString(Float) (- (Utilities|Time|GetGameTimeinSeconds) (- (/ (Math|Conversions|ToFloat(Integer) _impactframe_2) _returnvalue) (/ _framesbeforeimpact _returnvalue)))) "" "," (Utilities|String|ToString(Float) (Variables|/Game/Blueprints/BP_DisplayAngle.BP_DisplayAngle_C|GetAngleOfThigh_r_Subject (Utilities|Array|Get(acopy) (Utilities|Array|MakeArray _returnvalue_2)))) "," "" "" (Utilities|String|ToString(Float) (Variables|/Game/Blueprints/BP_DisplayAngle.BP_DisplayAngle_C|GetAngleOfCalf_r_Subject (Utilities|Array|Get(acopy) (Utilities|Array|MakeArray _returnvalue_2)))) "," "" "" (Utilities|String|ToString(Float) (Variables|/Game/Blueprints/BP_DisplayAngle.BP_DisplayAngle_C|GetAngleOfFoot_r_Subject (Utilities|Array|Get(acopy) (Utilities|Array|MakeArray _returnvalue_2)))) ",") true true)
      (Variables|Default|SetDataNames "")
      (Development|PrintString (Utilities|String|ToString(Integer) (Math|Float|Truncate (Utilities|Time|GetTimeSeconds))))
      (else
        (Development|PrintString "Ended")))
    (else
      (bind _isstarted (CallFunction|Start _impactframe _animationfps)))))

(fn ConstructionScript)

(fn Start
  (params (ImpactFrame :type Integer) (AnimationFPS :type Integer))
  (bind _returnvalue (Math|Conversions|ToFloat(Integer) AnimationFPS))
  (return (>= (Utilities|Time|GetGameTimeinSeconds) (- (/ (Math|Conversions|ToFloat(Integer) ImpactFrame) _returnvalue) (/ (Variables|Default|GetFramesBeforeImpact) _returnvalue)))))

(fn End
  (params (ImpactFrame :type Integer) (AnimationFPS :type Integer))
  (bind _returnvalue (Math|Conversions|ToFloat(Integer) AnimationFPS))
  (return (<= (Utilities|Time|GetGameTimeinSeconds) (+ (/ (Math|Conversions|ToFloat(Integer) ImpactFrame) _returnvalue) (/ (Variables|Default|GetFramesAfterImpact) _returnvalue)))))