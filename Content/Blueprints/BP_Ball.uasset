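; BP_Ball is a grabbable mixed-reality actor using UXT bounds control and generic manipulator components, with audio and visual grab feedback.
; Both components' start and end events share handlers that play grab or release sounds and swap the BoundControl material.
; The construction script temporarily zeroes actor rotation to fit BoundControl to the static mesh's bounds, then restores the transform and applies the visibility flag.
; BeginPlay disables BoundControl's collision.
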(event OnManipulationStarted(UxtBoundsControl)
  (params (Manipulator :type Uxt%20Bounds%20Control%20Component%20Object%20Reference) (AffordanceInfo :type Uxt%20Affordance%20Config%20Structure%20%28by%20ref%29) (GrabbedComponent :type Uxt%20Grab%20Target%20Component%20Object%20Reference))
  (Audio|PlaySoundatLocation (Variables|Default|GetGrabbedSound) (Transformation|GetActorLocation) "0, 0, 0" 1.0 1.0 0.0 0 0 0 0)
  (Rendering|Material|SetMaterial (Variables|Default|GetBoundControl) 0 (Variables|Default|GetBoundsGrabbedMaterial)))

(event OnManipulationEnded(UxtBoundsControl)
  (params (Manipulator :type Uxt%20Bounds%20Control%20Component%20Object%20Reference) (AffordanceInfo :type Uxt%20Affordance%20Config%20Structure%20%28by%20ref%29) (GrabbedComponent :type Uxt%20Grab%20Target%20Component%20Object%20Reference))
  (Audio|PlaySoundatLocation (Variables|Default|GetReleasedSound) (Transformation|GetActorLocation) "0, 0, 0" 1.0 1.0 0.0 0 0 0 0)
  (Rendering|Material|SetMaterial (Variables|Default|GetBoundControl) 0 (Variables|Default|GetBoundsMaterial)))

(event OnBeginGrab(UxtGenericManipulator)
  (params (Grabbable :type Uxt%20Grab%20Target%20Component%20Object%20Reference) (GrabPointer :type Uxt%20Grab%20Pointer%20Data%20Structure))
  (Audio|PlaySoundatLocation (Variables|Default|GetGrabbedSound) (Transformation|GetActorLocation) "0, 0, 0" 1.0 1.0 0.0 0 0 0 0)
  (Rendering|Material|SetMaterial (Variables|Default|GetBoundControl) 0 (Variables|Default|GetBoundsGrabbedMaterial)))

(event OnEndGrab(UxtGenericManipulator)
  (params (Grabbable :type Uxt%20Grab%20Target%20Component%20Object%20Reference) (GrabPointer :type Uxt%20Grab%20Pointer%20Data%20Structure))
  (Audio|PlaySoundatLocation (Variables|Default|GetReleasedSound) (Transformation|GetActorLocation) "0, 0, 0" 1.0 1.0 0.0 0 0 0 0)
  (Rendering|Material|SetMaterial (Variables|Default|GetBoundControl) 0 (Variables|Default|GetBoundsMaterial)))

(event EventBeginPlay
  (Collision|SetCollisionEnabled (Variables|Default|GetBoundControl) "NoCollision"))

(event Collision|EventActorBeginOverlap
  (params (OtherActor :type Actor%20Object%20Reference)))

(event EventTick
  (params (DeltaSeconds :type Float%20%28single-precision%29)))

(fn ConstructionScript
  (bind _staticmesh (Variables|Default|GetStaticMesh))
  (bind (_origin _boxextent) (Collision|GetComponentBounds _staticmesh))
  ;[1 1 1] Setup BoundControl scale
  (Variables|Default|SetDefaultActorTransform (Transformation|GetActorTransform))
  (Transformation|SetActorRotation "0, 0, 0")
  (Transformation|SetWorldTransform (Variables|Default|GetBoundControl) (Math|Transform|MakeTransform _origin (.Rotation (Math|Transform|BreakTransform (Transformation|GetWorldTransform _staticmesh))) (* _boxextent 2.0)) false false)
  (Transformation|SetActorTransform (Variables|Default|GetDefaultActorTransform))
  (Rendering|SetVisibility (Variables|Default|GetBoundControl) (Variables|Default|GetShowBoundControl) false))