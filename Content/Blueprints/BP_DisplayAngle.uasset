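; Actor that measures right-leg joint angles on a subject (Sub) and a teacher (Tea) character and adds Widget_Display to the viewport.
; Each Tick it feeds socket locations into TheAngleOf2Lines, storing hip, knee and ankle angles for each, then prints timing debug text.
; The angle helper holds a dot-product arccosine formula and Differencebetween2 an absolute-difference one, both apparently unwired.
; The difference helper is never called.
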(event EventBeginPlay
  (bind _returnvalue (UserInterface|CreateWidget "/Game/Widget/Widget_Display.Widget_Display_C"))
  (UserInterface|Viewport|AddtoViewport _returnvalue 0))

(event EventTick
  (params (DeltaSeconds :type Float%20%28single-precision%29))
  (bind _returnvalue (Utilities|Time|GetTimeSeconds))
  (bind _returnvalue_2 (/ 1.0 DeltaSeconds))
  (bind _outactors (Actor|GetAllActorsOfClass "/Game/Blueprints/Sub.Sub_C"))
  (if (Transformation|DoesSocketExist (Utilities|Array|Get(acopy) (Actor|GetComponentsByClass (Utilities|Array|Get(acopy) _outactors) "/Script/Engine.SceneComponent")) "calf_r")
    ;[1 1 1] 脊椎と大腿骨のなす角
    (Variables|Default|SetAngleOfThigh_r_Subject (Utilities|TheAngleOf2Lines (Transformation|GetSocketLocation (Utilities|Array|Get(acopy) (Actor|GetComponentsByClass (Utilities|Array|Get(acopy) _outactors) "/Script/Engine.SceneComponent")) "pelvis") (Transformation|GetSocketLocation (Utilities|Array|Get(acopy) (Actor|GetComponentsByClass (Utilities|Array|Get(acopy) _outactors) "/Script/Engine.SceneComponent")) "spine_01") (Transformation|GetSocketLocation (Utilities|Array|Get(acopy) (Actor|GetComponentsByClass (Utilities|Array|Get(acopy) _outactors) "/Script/Engine.SceneComponent")) "thigh_r") (Transformation|GetSocketLocation (Utilities|Array|Get(acopy) (Actor|GetComponentsByClass (Utilities|Array|Get(acopy) _outactors) "/Script/Engine.SceneComponent")) "calf_r")))
    ;[1 1 1] 大腿骨と脛骨のなす角
    (Variables|Default|SetAngleOfCalf_r_Subject (Utilities|TheAngleOf2Lines (Transformation|GetSocketLocation (Utilities|Array|Get(acopy) (Actor|GetComponentsByClass (Utilities|Array|Get(acopy) _outactors) "/Script/Engine.SceneComponent")) "calf_r") (Transformation|GetSocketLocation (Utilities|Array|Get(acopy) (Actor|GetComponentsByClass (Utilities|Array|Get(acopy) _outactors) "/Script/Engine.SceneComponent")) "thigh_r") (Transformation|GetSocketLocation (Utilities|Array|Get(acopy) (Actor|GetComponentsByClass (Utilities|Array|Get(acopy) _outactors) "/Script/Engine.SceneComponent")) "calf_r") (Transformation|GetSocketLocation (Utilities|Array|Get(acopy) (Actor|GetComponentsByClass (Utilities|Array|Get(acopy) _outactors) "/Script/Engine.SceneComponent")) "foot_r")))
    ;[1 1 1] 脛骨と踵骨のなす角
    (Variables|Default|SetAngleOfFoot_r_Subject (Utilities|TheAngleOf2Lines (Transformation|GetSocketLocation (Utilities|Array|Get(acopy) (Actor|GetComponentsByClass (Utilities|Array|Get(acopy) _outactors) "/Script/Engine.SceneComponent")) "foot_r") (Transformation|GetSocketLocation (Utilities|Array|Get(acopy) (Actor|GetComponentsByClass (Utilities|Array|Get(acopy) _outactors) "/Script/Engine.SceneComponent")) "calf_r") (Transformation|GetSocketLocation (Utilities|Array|Get(acopy) (Actor|GetComponentsByClass (Utilities|Array|Get(acopy) _outactors) "/Script/Engine.SceneComponent")) "foot_r") (Transformation|GetSocketLocation (Utilities|Array|Get(acopy) (Actor|GetComponentsByClass (Utilities|Array|Get(acopy) _outactors) "/Script/Engine.SceneComponent")) "ball_r")))
    (bind _outactors_2 (Actor|GetAllActorsOfClass "/Game/Blueprints/Tea.Tea_C"))
    (if (Transformation|DoesSocketExist (Utilities|Array|Get(acopy) (Actor|GetComponentsByClass (Utilities|Array|Get(acopy) _outactors_2) "/Script/Engine.SceneComponent")) "calf_r")
      ;[1 1 1] 脊椎と大腿骨のなす角
      (Variables|Default|SetAngleOfThigh_r_Teacher (Utilities|TheAngleOf2Lines (Transformation|GetSocketLocation (Utilities|Array|Get(acopy) (Actor|GetComponentsByClass (Utilities|Array|Get(acopy) _outactors_2) "/Script/Engine.SceneComponent")) "pelvis") (Transformation|GetSocketLocation (Utilities|Array|Get(acopy) (Actor|GetComponentsByClass (Utilities|Array|Get(acopy) _outactors_2) "/Script/Engine.SceneComponent")) "spine_01") (Transformation|GetSocketLocation (Utilities|Array|Get(acopy) (Actor|GetComponentsByClass (Utilities|Array|Get(acopy) _outactors_2) "/Script/Engine.SceneComponent")) "thigh_r") (Transformation|GetSocketLocation (Utilities|Array|Get(acopy) (Actor|GetComponentsByClass (Utilities|Array|Get(acopy) _outactors_2) "/Script/Engine.SceneComponent")) "calf_r")))
      ;[1 1 1] 大腿骨と脛骨のなす角
      (Variables|Default|SetAngleOfCalf_r_Teacher (Utilities|TheAngleOf2Lines (Transformation|GetSocketLocation (Utilities|Array|Get(acopy) (Actor|GetComponentsByClass (Utilities|Array|Get(acopy) _outactors_2) "/Script/Engine.SceneComponent")) "calf_r") (Transformation|GetSocketLocation (Utilities|Array|Get(acopy) (Actor|GetComponentsByClass (Utilities|Array|Get(acopy) _outactors_2) "/Script/Engine.SceneComponent")) "thigh_r") (Transformation|GetSocketLocation (Utilities|Array|Get(acopy) (Actor|GetComponentsByClass (Utilities|Array|Get(acopy) _outactors_2) "/Script/Engine.SceneComponent")) "calf_r") (Transformation|GetSocketLocation (Utilities|Array|Get(acopy) (Actor|GetComponentsByClass (Utilities|Array|Get(acopy) _outactors_2) "/Script/Engine.SceneComponent")) "foot_r")))
      ;[1 1 1] 脛骨と踵骨のなす角
      (Variables|Default|SetAngleOfFoot_r_Teacher (Utilities|TheAngleOf2Lines (Transformation|GetSocketLocation (Utilities|Array|Get(acopy) (Actor|GetComponentsByClass (Utilities|Array|Get(acopy) _outactors_2) "/Script/Engine.SceneComponent")) "foot_r") (Transformation|GetSocketLocation (Utilities|Array|Get(acopy) (Actor|GetComponentsByClass (Utilities|Array|Get(acopy) _outactors_2) "/Script/Engine.SceneComponent")) "calf_r") (Transformation|GetSocketLocation (Utilities|Array|Get(acopy) (Actor|GetComponentsByClass (Utilities|Array|Get(acopy) _outactors_2) "/Script/Engine.SceneComponent")) "foot_r") (Transformation|GetSocketLocation (Utilities|Array|Get(acopy) (Actor|GetComponentsByClass (Utilities|Array|Get(acopy) _outactors_2) "/Script/Engine.SceneComponent")) "ball_r")))
      (Development|PrintString (Utilities|String|Append "sec:" (Utilities|String|ToString(Float) _returnvalue) "," "FPS:" (Utilities|String|ToString(Float) _returnvalue_2) "," "Frame:" (Utilities|String|ToString(Float) (* _returnvalue _returnvalue_2))) true true "(R=0.000000,G=0.660000,B=1.000000,A=1.000000)" 1e+02))))

(fn ConstructionScript)